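; Enemy pawn that patrols four locations in a loop and reacts to targets sensed by AI perception.
; Sensing plays a ghost sound and writes target and sight flag to BPAI_Controller's Blackboard; losing it clears the flag and restarts patrol.
; Construction loads mesh and attack stats from DT_EnemiesData by class display name, then offsets the attack point by range.
; Attack only draws a debug box and damage text; its timer wiring is disconnected.
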(event `self.ReceiveBeginPlay`
  (`|AIMoveTo` self (`self.Location1`) null :!label _label
    (:`OnSuccess`
      (`|AIMoveTo` self (`self.Location2`) null
        (:`OnSuccess`
          (`|AIMoveTo` self (`self.Location3`) null
            (:`OnSuccess`
              (`|AIMoveTo` self (`self.Location4`) null
                (:`OnSuccess`
                  (goto _label))))))))))

(event `Attack`
  (bind _capsulecomponent (`self.CapsuleComponent`))
  (`KismetSystemLibrary.DrawDebugBox` (`SceneComponent.K2_GetComponentLocation` (`self.AttackSpawnLocation`)) (`KismetMathLibrary.MakeVector` (`self.AttackRange`) (* (`CapsuleComponent.GetScaledCapsuleRadius` _capsulecomponent) 2.0) (* (`CapsuleComponent.GetScaledCapsuleHalfHeight` _capsulecomponent) 2.0)) (struct :`A` 1.0) (`self.K2_GetActorRotation`) 2.0 1.0)
  (`KismetSystemLibrary.DrawDebugString` (`SceneComponent.K2_GetComponentLocation` (`self.AttackSpawnLocation`)) (`KismetStringLibrary.Conv_DoubleToString` (`self.Damage`)) null (struct :`R` 1.0 :`G` 0.255208 :`B` 0.919296 :`A` 1.0) 2.0))

(event `self.AIPerception.OnTargetPerceptionUpdated`
  (params (Actor :type "Actor Object Reference") (Stimulus :type "AIStimulus Structure"))
  (if (`.bSuccessfullySensed` (break `AIStimulus` Stimulus))
    (`GameplayStatics.PlaySound2D` "/Game/Sounds/GhostIdle.GhostIdle" 1.0 1.0 0.0 null null)
    (bind _asbpai_controller (cast `/Game/Enemies/BPAI_Controller` (`self.GetController`)))
    (bind _blackboard (`AIController.Blackboard` _asbpai_controller))
    (`BlackboardComponent.SetValueAsObject` _blackboard "TargetActor" Actor)
    (`BlackboardComponent.SetValueAsBool` _blackboard "IsPlayerInSigh" true)
    (else
      (`BlackboardComponent.SetValueAsBool` _blackboard "IsPlayerInSigh" false)
      (goto _label))))

(fn `LoadEnemyValues`
  (returns (Result :type Boolean))
  (bind _returnvalue (`|GetDataTableRow` "/Game/DataBase/DT_EnemiesData.DT_EnemiesData" (`KismetStringLibrary.Conv_StringToName` (`KismetSystemLibrary.GetClassDisplayName` (`GameplayStatics.GetObjectClass` self))))
    (:`then`
      (bind (_damage _attackrange _attackrate _mesh) (break `/Game/DataBase/FEnemyData` _returnvalue))
      (set `self.Damage` _damage)
      (set `self.AttackRange` _attackrange)
      (set `self.AttackRate` _attackrate)
      (`SkinnedMeshComponent.SetSkinnedAssetAndUpdate` (`self.Mesh`) _mesh true)
      (return true))
    (:`RowNotFound`
      (return false))))

(fn `UserConstructionScript`
  (bind _result (`self.LoadEnemyValues`))
  (if _result
    (`SceneComponent.K2_SetRelativeLocation` (`self.AttackSpawnLocation`) (`KismetMathLibrary.MakeVector` (/ (`self.AttackRange`) 2.0)) false false)))