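; BP_Enemy_2 is an enemy Blueprint that reports what it perceives to its AI controller's Blackboard.
; When AI Perception senses an actor, it casts its controller to BPAI_Controller, stores the actor as TargetActor and sets IsPlayerInSigh true, with no actor type check.
; Failed sensing sets that flag false through the success branch's cast result, leaving TargetActor unchanged.
; A Destination location write exists but is disconnected.
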(event `self.ReceiveBeginPlay`)

(event `self.AIPerception_0.OnTargetPerceptionUpdated`
  (params (Actor :type "Actor Object Reference") (Stimulus :type "AIStimulus Structure"))
  (if (`.bSuccessfullySensed` (break `AIStimulus` Stimulus))
    (bind _asbpai_controller (cast `/Game/Enemies/BPAI_Controller` (`self.GetController`)))
    (bind _blackboard (`AIController.Blackboard` _asbpai_controller))
    (`BlackboardComponent.SetValueAsObject` _blackboard "TargetActor" Actor)
    (`BlackboardComponent.SetValueAsBool` _blackboard "IsPlayerInSigh" true)
    (else
      (`BlackboardComponent.SetValueAsBool` _blackboard "IsPlayerInSigh" false))))

(fn `UserConstructionScript`)