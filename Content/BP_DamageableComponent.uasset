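; Damageable component that tracks a time value, CurrentTime, as the health of whatever owns it.
; On BeginPlay it fills CurrentTime to MaxTime and broadcasts OnDamage with zero damage.
; GetDamage sets CurrentTime to the incoming damage minus CurrentTime (not the reverse), clamped between zero and MaxTime.
; It then broadcasts OnDamage with the new value, and OnDeath when that value is zero.
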(event `self.ReceiveBeginPlay`
  (bind _output_get (set `self.CurrentTime` (`self.MaxTime`)))
  (`self.OnDamage` 0 _output_get))

(fn `GetDamage`
  (params (NewDamage :type Integer))
  (bind _currenttime (`self.CurrentTime`))
  (bind _output_get (set `self.CurrentTime` (`KismetMathLibrary.Clamp` (- NewDamage _currenttime) 0 (`self.MaxTime`))))
  (`self.OnDamage` NewDamage _currenttime)
  (if (== _output_get 0)
    (`self.OnDeath`)))